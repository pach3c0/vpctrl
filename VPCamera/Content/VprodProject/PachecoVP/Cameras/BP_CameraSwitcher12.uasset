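; Virtual production camera actor that plays four recorded A-to-B moves, each toggled forward or reverse by keys 1–4.
; The construction script records the actor's transform, duration and lens overrides into the active path when GravarA or GravarB is set.
; Duration-scaled timelines lerp the transform; only path 1 also animates focal length and manual focus.
; Tick copies Cam1's transform, FOV and focus distance to a SceneCaptureComponent2D.
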(event `self.ReceiveBeginPlay`)

(event `self.ReceiveTick`
  (params (DeltaSeconds :type "Float (single-precision)"))
  (bind _cam1 (`self.Cam1`))
  (bind _scenecapturecomponent2d (`self.SceneCaptureComponent2D`))
  (`SceneComponent.K2_SetWorldLocation` _scenecapturecomponent2d (`SceneComponent.K2_GetComponentLocation` _cam1) false false)
  (`SceneComponent.K2_SetWorldRotation` _scenecapturecomponent2d (`SceneComponent.K2_GetComponentRotation` _cam1) false false)
  (set `SceneCaptureComponent2D.FOVAngle` (`CameraComponent.FieldOfView` _cam1) _scenecapturecomponent2d)
  (setmembers `PostProcessSettings` :`StructRef` (`SceneCaptureComponent2D.PostProcessSettings` _scenecapturecomponent2d) :`DepthOfFieldFocalDistance` (`CineCameraComponent.CurrentFocusDistance` _cam1)))

(event `Key|One`
  (params (Key :type "Key Structure"))
  (bind (_pointa _pointb _duration _focallengtha _focusdistancea _focallengthb _focusdistanceb) (break `/VPCamera/VprodProject/PachecoVP/S_CameraPath` (`|GetArrayItem` (`self.Paths`))))
  (:`Pressed`
    (`/Engine/EditorBlueprintResources/StandardMacros.FlipFlop`
      (:`A`
        (`TimelineComponent.SetPlayRate` (`self.TL_Path1`) (/ 1.0 _duration))
        (bind (_direction _alpha) (`Timeline|TL_Path1` :!via `PlayFromStart` :!label _label)
          (:`Update`
            (`self.K2_SetActorTransform` self (`KismetMathLibrary.TLerp` _pointa _pointb _alpha) false false)
            (set `CineCameraComponent.CurrentFocalLength` (`KismetMathLibrary.Lerp` _focallengtha _focallengthb _alpha) (`self.Cam1`))
            (set `CineCameraComponent.FocusSettings` (make `CameraFocusSettings` "Manual" (`KismetMathLibrary.Lerp` _focusdistancea _focusdistanceb _alpha)) (`self.Cam1`)))
          (:`Finished`
            (set `self.IsMoving` false))))
      (:`B`
        (goto _label :!via `Reverse`)))))

(event `Key|Two`
  (params (Key :type "Key Structure"))
  (bind (_pointa _pointb _duration) (break `/VPCamera/VprodProject/PachecoVP/S_CameraPath` (`|GetArrayItem` (`self.Paths`) 1)))
  (:`Pressed`
    (`/Engine/EditorBlueprintResources/StandardMacros.FlipFlop`
      (:`A`
        (`TimelineComponent.SetPlayRate` (`self.TL_Path2`) (/ 1.0 _duration))
        (bind (_direction _alpha) (`Timeline|TL_Path2` :!via `PlayFromStart` :!label _label_2)
          (:`Update`
            (`self.K2_SetActorTransform` self (`KismetMathLibrary.TLerp` _pointa _pointb _alpha) false false))
          (:`Finished`
            (set `self.IsMoving` false))))
      (:`B`
        (goto _label_2 :!via `Reverse`)))))

(event `Key|Three`
  (params (Key :type "Key Structure"))
  (bind (_pointa _pointb _duration) (break `/VPCamera/VprodProject/PachecoVP/S_CameraPath` (`|GetArrayItem` (`self.Paths`) 2)))
  (:`Pressed`
    (`/Engine/EditorBlueprintResources/StandardMacros.FlipFlop`
      (:`A`
        (`TimelineComponent.SetPlayRate` (`self.TL_Path3`) (/ 1.0 _duration))
        (bind (_direction _alpha) (`Timeline|TL_Path3` :!via `PlayFromStart` :!label _label_3)
          (:`Update`
            (`self.K2_SetActorTransform` self (`KismetMathLibrary.TLerp` _pointa _pointb _alpha) false false))
          (:`Finished`
            (set `self.IsMoving` false))))
      (:`B`
        (goto _label_3 :!via `Reverse`)))))

(event `Key|Four`
  (params (Key :type "Key Structure"))
  (bind (_pointa _pointb _duration) (break `/VPCamera/VprodProject/PachecoVP/S_CameraPath` (`|GetArrayItem` (`self.Paths`) 3)))
  (:`Pressed`
    (`/Engine/EditorBlueprintResources/StandardMacros.FlipFlop`
      (:`A`
        (`TimelineComponent.SetPlayRate` (`self.TL_Path4`) (/ 1.0 _duration))
        (bind (_direction _alpha) (`Timeline|TL_Path4` :!via `PlayFromStart` :!label _label_4)
          (:`Update`
            (`self.K2_SetActorTransform` self (`KismetMathLibrary.TLerp` _pointa _pointb _alpha) false false))
          (:`Finished`
            (set `self.IsMoving` false))))
      (:`B`
        (goto _label_4 :!via `Reverse`)))))

(fn `UserConstructionScript`
  (bind _focallengthoverride (`self.FocalLengthOverride`))
  (bind _focusdistanceoverride (`self.FocusDistanceOverride`))
  (bind _activepath (`self.ActivePath`))
  (bind _activepath_2 (`self.ActivePath`))
  (bind (_pointa _pointb _duration _focallengtha _focusdistancea) (break `/VPCamera/VprodProject/PachecoVP/S_CameraPath` (`|GetArrayItem` (`self.Paths`) _activepath)))
  (bind (_pointa_2 _pointb_2 _duration_2 _focallengtha_2 _focusdistancea_2 _focallengthb _focusdistanceb) (break `/VPCamera/VprodProject/PachecoVP/S_CameraPath` (`|GetArrayItem` (`self.Paths`) _activepath_2)))
  (if (`self.GravarA`)
    (`KismetArrayLibrary.Array_Set` (`self.Paths`) _activepath_2 (make `/VPCamera/VprodProject/PachecoVP/S_CameraPath` (`self.GetTransform`) _pointb_2 (`self.Duration`) _focallengthoverride _focusdistanceoverride _focallengthb _focusdistanceb))
    (elif (`self.GravarB`)
      (`KismetArrayLibrary.Array_Set` (`self.Paths`) _activepath (make `/VPCamera/VprodProject/PachecoVP/S_CameraPath` _pointa (`self.GetTransform`) (`self.Duration`) _focallengtha _focusdistancea _focallengthoverride _focusdistanceoverride)))))